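; BP_Valve is a valve that spins when its HitPlayer event fires and then notifies a target actor.
; A timeline interpolates the static mesh's relative rotation from StartRotation to EndRotation, then clears Spinning and calls ValveSpunMessage on TargetActor.
; HitPlayer checks Spinning before playing, but nothing shown sets that flag to true.
; FetchMoveInput is a stub returning zero input.
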(event `/Game/Blueprints/Interfaces/BPI_Player.Hit Player`
  (params (`Damage Value` :type "Float (double-precision)") (`Knockback Value` :type "Float (double-precision)") (`Hitting Actor` :type "Actor Object Reference"))
  (if (not (`self.Spinning?`))
    (bind (_direction _alpha) (`Timeline|Timeline` :!via `PlayFromStart`)
      (:`Update`
        (`SceneComponent.K2_SetRelativeRotation` (`self.StaticMesh`) (`KismetMathLibrary.RLerp` (`self.StartRotation`) (`self.EndRotation`) _alpha) false false))
      (:`Finished`
        (set `self.Spinning?` false)
        (message `/Game/Blueprints/Interfaces/BPI_Valve.ValveSpun` (`self.TargetActor`))))))

(fn `FetchMoveInput`
  (returns (X :type "Float (double-precision)") (Y :type "Float (double-precision)"))
  (return 0.0 0.0))

(fn `UserConstructionScript`)