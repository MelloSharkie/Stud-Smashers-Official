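; BP_Boulder is a boulder actor that releases a physics-driven sphere in a repeating cycle.
; After an initial delay, each cycle plays a wide-radius rumble camera shake and a loud 2D sound as a warning.
; A few seconds later it teleports the sphere to the actor's location and enables physics.
; It later disables physics and loops back to the rumble, reusing the same sphere rather than spawning new ones.
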(event `self.ReceiveBeginPlay`
  (bind _sphere (`self.Sphere`))
  (`KismetSystemLibrary.Delay` 5.0)
  (`GameplayStatics.PlayWorldCameraShake` "/Game/Blueprints/CameraShake/CS_BoulderRumble.CS_BoulderRumble_C" (`self.K2_GetActorLocation`) 40000.0 40000.0 :!label _label)
  (`GameplayStatics.PlaySound2D` "/Game/Sound/423781__someonecool15__lego-bricks-dump-1.423781__someonecool15__lego-bricks-dump-1" 5.0 1.0 0.0 null null)
  (`KismetSystemLibrary.Delay` 3.0)
  (`SceneComponent.K2_SetWorldLocation` _sphere (`self.K2_GetActorLocation`) false true)
  (`PrimitiveComponent.SetSimulatePhysics` _sphere true)
  (`KismetSystemLibrary.Delay` 20.0)
  (`PrimitiveComponent.SetSimulatePhysics` (`self.Sphere`) false)
  (goto _label))

(fn `UserConstructionScript`)