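; BP_PortalButton is a LEGO-style pressure button that triggers spike walls when a player overlaps its box.
; A press swaps the material on four meshes, calls TriggerWall on each SpikeWallArray entry and runs a timeline that offsets the button downward.
; Timeline completion restores the red material and re-arms it.
; Triggered is set before the BPI_Player interface check, so a non-player overlap leaves it latched.
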(event `self.Box.OnComponentBeginOverlap`
  (params (OverlappedComponent :type "PrimitiveComponent Object Reference") (OtherActor :type "Actor Object Reference") (OtherComp :type "PrimitiveComponent Object Reference") (OtherBodyIndex :type Integer) (bFromSweep :type Boolean) (SweepResult :type "HitResult Structure (by ref)"))
  (if (not (`self.Triggered?`))
    (set `self.Triggered?` true)
    (if (`KismetSystemLibrary.DoesImplementInterface` OtherActor "/Game/Blueprints/Interfaces/BPI_Player.BPI_Player_C")
      (`PrimitiveComponent.SetMaterial` (`self.StaticMesh1`) 0 "/Game/Assets/Arenas/Ninjago/BaseModels/NewMeshes/MAT_LEGOBrick_003.MAT_LEGOBrick_003")
      (`PrimitiveComponent.SetMaterial` (`self.StaticMesh2`) 0 "/Game/Assets/Arenas/Ninjago/BaseModels/NewMeshes/MAT_LEGOBrick_003.MAT_LEGOBrick_003")
      (`PrimitiveComponent.SetMaterial` (`self.StaticMesh3`) 0 "/Game/Assets/Arenas/Ninjago/BaseModels/NewMeshes/MAT_LEGOBrick_003.MAT_LEGOBrick_003")
      (`PrimitiveComponent.SetMaterial` (`self.StaticMesh4`) 0 "/Game/Assets/Arenas/Ninjago/BaseModels/NewMeshes/MAT_LEGOBrick_003.MAT_LEGOBrick_003")
      (for _array_element (`self.SpikeWallArray`)
        (`/Game/Blueprints/BP_SpikeWall.TriggerWall` _array_element))
      (set `self.Button Location` (`self.K2_GetActorLocation`))
      (bind (_direction _alpha) (`Timeline|ButtonTimeline` :!via `PlayFromStart`)
        (:`Update`
          (`self.K2_SetActorRelativeLocation` (`KismetMathLibrary.VLerp` (`self.Button Location`) (+ (`self.Button Location`) (0.0 0.0 -7.123502)) _alpha)))
        (:`Finished`
          (set `self.Triggered?` false)
          (`PrimitiveComponent.SetMaterial` (`self.StaticMesh1`) 0 "/Game/Assets/Materials/MI_LEGOBrick_Red.MI_LEGOBrick_Red")
          (`PrimitiveComponent.SetMaterial` (`self.StaticMesh2`) 0 "/Game/Assets/Materials/MI_LEGOBrick_Red.MI_LEGOBrick_Red")
          (`PrimitiveComponent.SetMaterial` (`self.StaticMesh3`) 0 "/Game/Assets/Materials/MI_LEGOBrick_Red.MI_LEGOBrick_Red")
          (`PrimitiveComponent.SetMaterial` (`self.StaticMesh4`) 0 "/Game/Assets/Materials/MI_LEGOBrick_Red.MI_LEGOBrick_Red"))))))

(fn `UserConstructionScript`)