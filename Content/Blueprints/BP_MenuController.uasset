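; Player controller for the multiplayer menus, showing the lobby, loading screen and podium widgets with UI-only input.
; Initial setup loads the profile save, creating it if missing, then passes it through ServerUpdateLobby so BP_MainMenuGameMode refreshes the lobby.
; Events update lobby names, store the player number in the GameInstance, and end the session by returning to the main menu level.
; Each widget is created on first use and its reference reused.
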(event `Create Load Screen`
  (`self.UI_ShowLoadScreen`))

(event `self.ReceiveBeginPlay`
  (if (`self.IsLocalController`)
    (set `self.bShowMouseCursor` true)
    (`WidgetBlueprintLibrary.SetInputMode_UIOnlyEx` self null)))

(event `EndClientSession`
  (`DestroySessionCallbackProxy.DestroySession` self
    (:`then`
      (`GameplayStatics.OpenLevel` "LV_MainMenu"))))

(event `Create Lobby Menu`
  (`self.UI_ShowLobbyMenu`))

(event `InitialSetupEvent`
  (`self.LoadSavedProfile`)
  (`self.Server Update Lobby` (`self.Player Profile Info`)))

(event `Server Update Lobby`
  (params (`Player Profile` :type "/Game/SavedData/STR_PlayerProfile Structure"))
  (set `self.Player Profile Info` `Player Profile`)
  (bind _asbp_main_menu_game_mode (cast `/Game/Blueprints/BP_MainMenuGameMode` (`GameplayStatics.GetGameMode`)))
  (`/Game/Blueprints/BP_MainMenuGameMode.UpdateLobbyEvent` _asbp_main_menu_game_mode true))

(event `UpdatePlayerNames`
  (params (PlayerProfiles :type "Array of /Game/SavedData/STR_PlayerProfile Structure"))
  (bind _lobby_menu_reference (`self.Lobby Menu Reference`))
  (`/Engine/EditorBlueprintResources/StandardMacros.IsValid` _lobby_menu_reference
    (:`Is Valid`
      (`/Game/Blueprints/Widgets/WI_LobbyMenu.ClearPlayerNames` _lobby_menu_reference)
      (`/Game/Blueprints/Widgets/WI_LobbyMenu.UpdatePlayerNames` _lobby_menu_reference PlayerProfiles))))

(event `Update Player Number`
  (params (`Player Number` :type Integer))
  (bind _asbp_game_instance (cast `/Game/Blueprints/BP_GameInstance` (`GameplayStatics.GetGameInstance`)))
  (`/Game/Blueprints/BP_GameInstance.Set Player Number` _asbp_game_instance `Player Number`))

(event `Create Podium Menu`
  (`self.UI_ShowPodiumMenu`))

(fn `LoadSavedProfile`
  (locals (LocalSlotName :type String :default "Player Profile Slot"))
  (bind _returnvalue (`GameplayStatics.DoesSaveGameExist` (`local.LocalSlotName`)))
  (if (not _returnvalue)
    (bind _returnvalue_2 (`GameplayStatics.CreateSaveGameObject` "/Game/SavedData/SG_PlayerProfile.SG_PlayerProfile_C"))
    (`GameplayStatics.SaveGameToSlot` _returnvalue_2 (`local.LocalSlotName`)))
  (bind _returnvalue_3 (`GameplayStatics.LoadGameFromSlot` (`local.LocalSlotName`)))
  (bind _assg_player_profile (cast `/Game/SavedData/SG_PlayerProfile` _returnvalue_3))
  (set `self.Player Profile Info` (`/Game/SavedData/SG_PlayerProfile.Player Profile` _assg_player_profile))
  (return))

(fn `UI_ShowLoadScreen`
  (`WidgetLayoutLibrary.RemoveAllWidgets`)
  (`/Engine/EditorBlueprintResources/StandardMacros.IsValid` (`self.LoadScreenReference`)
    (:`Is Valid`
      _)
    (:`Is Not Valid`
      (bind _returnvalue (`|CreateWidget` "/Game/Blueprints/Widgets/WI_LoadingScreen.WI_LoadingScreen_C" self))
      (set `self.LoadScreenReference` _returnvalue)))
  (`UserWidget.AddToViewport` (`self.LoadScreenReference`) 0)
  (return))

(fn `UI_ShowLobbyMenu`
  (`/Engine/EditorBlueprintResources/StandardMacros.IsValid` (`self.Lobby Menu Reference`)
    (:`Is Valid`
      _)
    (:`Is Not Valid`
      (bind _returnvalue (`|CreateWidget` "/Game/Blueprints/Widgets/WI_LobbyMenu.WI_LobbyMenu_C" self))
      (set `self.Lobby Menu Reference` _returnvalue)))
  (`UserWidget.AddToViewport` (`self.Lobby Menu Reference`) 0)
  (return))

(fn `UI_ShowPodiumMenu`
  (`/Engine/EditorBlueprintResources/StandardMacros.IsValid` (`self.Podium Menu Reference`)
    (:`Is Valid`
      _)
    (:`Is Not Valid`
      (bind _returnvalue (`|CreateWidget` "/Game/Blueprints/Widgets/WI_Podium.WI_Podium_C" self))
      (set `self.Podium Menu Reference` _returnvalue)))
  (`UserWidget.AddToViewport` (`self.Podium Menu Reference`) 0)
  (`KismetSystemLibrary.PrintString` "create podium menu - uishowpodiummenu - menucontroller" true true (struct :`G` 0.66 :`B` 1.0 :`A` 1.0) 5.0)
  (return))

(fn `UserConstructionScript`)