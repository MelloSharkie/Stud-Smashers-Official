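; BP_SpikeWall is a trap wall that calls TriggerDeath on any BP_ThirdPersonCharacter overlapping its Box.
; TriggerWall calls TriggerWallOnClients, where a Timeline slides StaticMesh1 along local Y, then re-arms after a short delay.
; TriggerWall has its own longer cooldown on the same CanBeTriggered flag.
; It clears that flag before calling TriggerWallOnClients, so the slide is skipped on the calling instance.
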(event `TriggerWall On Clients`
  (if (`self.CanBeTriggered`)
    (set `self.CanBeTriggered` false)
    (bind (_direction _newtrack_0) (`Timeline|Timeline` :!via `PlayFromStart`)
      (:`Update`
        (`SceneComponent.K2_SetRelativeLocation` (`self.StaticMesh1`) (`KismetMathLibrary.VLerp` (0.0 0.0 0.0) (0.0 560.0 0.0) _newtrack_0) false false))
      (:`Finished`
        (`KismetSystemLibrary.Delay` 2.0)
        (set `self.CanBeTriggered` true)))))

(event `TriggerWall`
  (if (`self.CanBeTriggered`)
    (set `self.CanBeTriggered` false)
    (`self.TriggerWall On Clients`)
    (`KismetSystemLibrary.Delay` 7.0)
    (set `self.CanBeTriggered` true)))

(event `self.Box.OnComponentBeginOverlap`
  (params (OverlappedComponent :type "PrimitiveComponent Object Reference") (OtherActor :type "Actor Object Reference") (OtherComp :type "PrimitiveComponent Object Reference") (OtherBodyIndex :type Integer) (bFromSweep :type Boolean) (SweepResult :type "HitResult Structure (by ref)"))
  (bind _asbp_third_person_character (cast `/Game/Blueprints/BP_ThirdPersonCharacter` OtherActor))
  (`/Game/Blueprints/BP_ThirdPersonCharacter.Trigger Death` _asbp_third_person_character))

(fn `UserConstructionScript`)