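; BP_Sewage is a sewage burst hazard that periodically knocks players back without dealing damage.
; A delay loop builds pressure while inactive, valve spins add extra increments, and a full count triggers an eruption.
; A timeline ramps up a warning light before the Niagara burst briefly activates the hazard.
; The capsule pushes players already inside at eruption, and those entering during it less strongly, through BPI_Player.
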(event `self.ReceiveBeginPlay`
  (`KismetSystemLibrary.Delay` 8.0)
  (`KismetSystemLibrary.Delay` 3.0 :!label _label)
  (if (`self.Active?`) :!label _label_2
    (goto _label)
    (else
      (bind _result (`/Engine/EditorBlueprintResources/StandardMacros.IncrementInt` (`self.PressureBuilt`))
        (:`  `
          (if (>= _result 10)
            (set `self.PressureBuilt` 0)
            (`self.ActivateSewage`)
            (goto _label)
            (else
              (goto _label))))))))

(event `self.ValveSpun`
  (goto _label_2))

(event `ActivateSewage`
  (`SceneComponent.SetVisibility` (`self.PointLight`) true false)
  (bind (_direction _alpha) (`Timeline|LightIntensityTimeline` :!via `PlayFromStart`)
    (:`Update`
      (`LightComponent.SetIntensity` (`self.PointLight`) (`KismetMathLibrary.Lerp` 0.0 100000.0 _alpha)))
    (:`Finished`
      (`ActorComponent.Activate` (`self.Niagara`) true)
      (`KismetSystemLibrary.Delay` 0.2)
      (set `self.Active?` true)
      (`self.CheckForOverlappingActors`)
      (`KismetSystemLibrary.Delay` 1.0)
      (`SceneComponent.SetVisibility` (`self.PointLight`) false false)
      (`ActorComponent.Deactivate` (`self.Niagara`))
      (set `self.Active?` false))))

(event `CheckForOverlappingActors`
  (for _array_element (`PrimitiveComponent.GetOverlappingActors` (`self.Capsule`) null)
    (if (`KismetSystemLibrary.DoesImplementInterface` _array_element "/Game/Blueprints/Interfaces/BPI_Player.BPI_Player_C")
      (message `/Game/Blueprints/Interfaces/BPI_Player.Hit Player` _array_element 0.0 5000.0 self))))

(event `self.Capsule.OnComponentBeginOverlap`
  (params (OverlappedComponent :type "PrimitiveComponent Object Reference") (OtherActor :type "Actor Object Reference") (OtherComp :type "PrimitiveComponent Object Reference") (OtherBodyIndex :type Integer) (bFromSweep :type Boolean) (SweepResult :type "HitResult Structure (by ref)"))
  (if (`KismetSystemLibrary.DoesImplementInterface` OtherActor "/Game/Blueprints/Interfaces/BPI_Player.BPI_Player_C")
    (if (`self.Active?`)
      (message `/Game/Blueprints/Interfaces/BPI_Player.Hit Player` OtherActor 0.0 2000.0 self))))

(fn `UserConstructionScript`)