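; BP_NinjagoObstacle01 is a Ninjago spinning hazard that kills the player character on contact.
; The Spin event plays a startup montage, sets CanSpin when it blends out or completes, then plays a stopping montage after a fixed delay.
; Two box volumes call TriggerDeath on any overlapping BP_ThirdPersonCharacter, without checking the spin state.
; CanSpin is never cleared or read in this graph.
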(event `/Game/Blueprints/Interfaces/BPI_Ninjago.Spin`
  (`|PlayMontage` (`self.SkeletalMesh`) "/Game/Assets/Arenas/Ninjago/Hazards/Anims/Ninjago_Spinny_Alternative_Anim_AltHazardStartup_Montage.Ninjago_Spinny_Alternative_Anim_AltHazardStartup_Montage"
    (:`OnCompleted`
      _)
    (:`OnBlendOut`
      _))
  (set `self.Can Spin?` true)
  (`KismetSystemLibrary.Delay` 15.0)
  (`|PlayMontage` (`self.SkeletalMesh`) "/Game/Assets/Arenas/Ninjago/Hazards/SKM/AlternateAnims_Anim_AltHazardStopping_Montage.AlternateAnims_Anim_AltHazardStopping_Montage"))

(event `self.Box1.OnComponentBeginOverlap`
  (params (OverlappedComponent :type "PrimitiveComponent Object Reference") (OtherActor :type "Actor Object Reference") (OtherComp :type "PrimitiveComponent Object Reference") (OtherBodyIndex :type Integer) (bFromSweep :type Boolean) (SweepResult :type "HitResult Structure (by ref)"))
  (bind _asbp_third_person_character (cast `/Game/Blueprints/BP_ThirdPersonCharacter` OtherActor))
  (`/Game/Blueprints/BP_ThirdPersonCharacter.Trigger Death` _asbp_third_person_character))

(event `self.Box.OnComponentBeginOverlap`
  (params (OverlappedComponent :type "PrimitiveComponent Object Reference") (OtherActor :type "Actor Object Reference") (OtherComp :type "PrimitiveComponent Object Reference") (OtherBodyIndex :type Integer) (bFromSweep :type Boolean) (SweepResult :type "HitResult Structure (by ref)"))
  (bind _asbp_third_person_character (cast `/Game/Blueprints/BP_ThirdPersonCharacter` OtherActor))
  (`/Game/Blueprints/BP_ThirdPersonCharacter.Trigger Death` _asbp_third_person_character))

(fn `UserConstructionScript`)