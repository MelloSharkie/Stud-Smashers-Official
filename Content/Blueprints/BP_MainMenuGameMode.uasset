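; Game mode for the menu levels that tracks connected menu controllers and sets up each player's lobby or podium menu.
; New players are handled by current level name: the lobby also runs initial setup and assigns an incrementing player number, which logouts do not decrement.
; UpdateLobbyEvent, also triggered on logout, copies each controller's profile to its PlayerState and sends the full profile list to every controller.
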(event `self.K2_OnLogout`
  (params (ExitingController :type "Controller Object Reference"))
  (bind _asbp_menu_controller (cast `/Game/Blueprints/BP_MenuController` ExitingController))
  (`KismetArrayLibrary.Array_RemoveItem` (`self.AllConnectedPlayers`) _asbp_menu_controller)
  (`self.UpdateLobbyEvent` true))

(event `self.ReceiveBeginPlay`
  (set `self.LastPlayerNumber` 0))

(event `self.HandleStartingNewPlayer`
  (params (NewPlayer :type "PlayerController Object Reference"))
  (bind _allconnectedplayers (`self.AllConnectedPlayers`))
  (bind _lastplayernumber (`self.LastPlayerNumber`))
  (bind _returnvalue (`GameplayStatics.GetCurrentLevelName` true))
  (switch `string` _returnvalue
    (:`LV_Lobby`
      (bind _asbp_menu_controller (cast `/Game/Blueprints/BP_MenuController` NewPlayer))
      (`KismetArrayLibrary.Array_Add` _allconnectedplayers _asbp_menu_controller)
      (`/Game/Blueprints/BP_MenuController.Create Lobby Menu` _asbp_menu_controller)
      (`/Game/Blueprints/BP_MenuController.InitialSetupEvent` _asbp_menu_controller)
      (`/Game/Blueprints/BP_MenuController.Update Player Number` _asbp_menu_controller _lastplayernumber)
      (`/Engine/EditorBlueprintResources/StandardMacros.IncrementInt` _lastplayernumber))
    (:`LV_Podium`
      (bind _asbp_menu_controller_2 (cast `/Game/Blueprints/BP_MenuController` NewPlayer))
      (`KismetArrayLibrary.Array_Add` _allconnectedplayers _asbp_menu_controller_2)
      (`/Game/Blueprints/BP_MenuController.Create Podium Menu` _asbp_menu_controller_2))))

(event `UpdateLobbyEvent`
  (params (PlayerNames :type Boolean))
  (if PlayerNames
    (`KismetArrayLibrary.Array_Clear` (`self.AllPlayerProfiles`))
    (for _array_element (`self.AllConnectedPlayers`)
      (bind _player_profile_info (`/Game/Blueprints/BP_MenuController.Player Profile Info` _array_element))
      (`KismetArrayLibrary.Array_Add` (`self.AllPlayerProfiles`) _player_profile_info)
      (bind _asbp_playerstate (cast `/Game/Blueprints/BP_Playerstate` (`Controller.PlayerState` _array_element)))
      (set `/Game/Blueprints/BP_Playerstate.Player Profile` _player_profile_info _asbp_playerstate))
    (for _array_element_2 (`self.AllConnectedPlayers`)
      (if PlayerNames
        (`/Game/Blueprints/BP_MenuController.UpdatePlayerNames` _array_element_2 (`self.AllPlayerProfiles`))))))

(fn `UserConstructionScript`)