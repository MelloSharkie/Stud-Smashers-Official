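; BP_ScoobyDooKnight is a knight hazard that periodically swings a halberd and kills player characters it hits.
; The server runs an endless loop from BeginPlay, waiting a random interval, then playing a montage through a server-to-clients event pair.
; A delayed, short Attacking window follows each montage start.
; Halberd overlaps that begin during that window call TriggerDeath on BP_ThirdPersonCharacter actors.
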(event `Play Montage On Clients`
  (params (`Skeletal Mesh Ref` :type "SkeletalMeshComponent Object Reference") (`Anim Montage Ref` :type "AnimMontage Object Reference"))
  (`|PlayMontage` `Skeletal Mesh Ref` `Anim Montage Ref`))

(event `Play Montage On Server`
  (params (`Skeletal Mesh Ref` :type "SkeletalMeshComponent Object Reference") (`Anim Montage Ref` :type "AnimMontage Object Reference"))
  (`self.Play Montage On Clients` `Skeletal Mesh Ref` `Anim Montage Ref`))

(event `self.ReceiveBeginPlay`
  (if (`KismetSystemLibrary.IsServer`)
    (`KismetSystemLibrary.Delay` (`KismetMathLibrary.RandomFloatInRange` 20.0 60.0) :!label _label)
    (`self.Play Montage On Server` (`self.SkeletalMesh`) (`self.Montage to Play`))
    (`KismetSystemLibrary.Delay` 1.0)
    (set `self.Attacking` true)
    (`KismetSystemLibrary.Delay` 1.0)
    (set `self.Attacking` false)
    (goto _label)))

(event `self.Halberd.OnComponentBeginOverlap`
  (params (OverlappedComponent :type "PrimitiveComponent Object Reference") (OtherActor :type "Actor Object Reference") (OtherComp :type "PrimitiveComponent Object Reference") (OtherBodyIndex :type Integer) (bFromSweep :type Boolean) (SweepResult :type "HitResult Structure (by ref)"))
  (if (`self.Attacking`)
    (bind _asbp_third_person_character (cast `/Game/Blueprints/BP_ThirdPersonCharacter` OtherActor))
    (`/Game/Blueprints/BP_ThirdPersonCharacter.Trigger Death` _asbp_third_person_character)))

(fn `UserConstructionScript`)