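; BP_NinjagoObstacle02 is a spinning hazard that knocks third-person characters away on contact.
; Spin plays a startup montage, then on blend-out or completion sets CanSpin and runs a timeline that drives Speed.
; When the timeline finishes, a stopping montage plays and CanSpin clears after a short delay.
; Two capsule overlaps launch the character away from the actor's location, with a strong horizontal push and weaker vertical component.
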(event `/Game/Blueprints/Interfaces/BPI_Ninjago.Spin`
  (`|PlayMontage` (`self.SkeletalMesh1`) "/Game/Assets/Arenas/Ninjago/Hazards/Anims/spinnyanims_Anim_CenterHazardStartup_Montage.spinnyanims_Anim_CenterHazardStartup_Montage"
    (:`OnCompleted`
      _)
    (:`OnBlendOut`
      _))
  (set `self.Can Spin?` true)
  (bind (_direction _speed) (`Timeline|Timeline` :!via `PlayFromStart`)
    (:`Update`
      (set `self.Speed` _speed))
    (:`Finished`
      (`|ExecutionSequence`
        (:`then_0`
          (`|PlayMontage` (`self.SkeletalMesh1`) "/Game/Assets/Arenas/Ninjago/Hazards/Anims/spinnyanims_Anim_CenterHazardStopping_Montage.spinnyanims_Anim_CenterHazardStopping_Montage"))
        (:`then_1`
          (`KismetSystemLibrary.Delay` 0.2)
          (set `self.Can Spin?` false))))))

(event `self.Capsule.OnComponentBeginOverlap`
  (params (OverlappedComponent :type "PrimitiveComponent Object Reference") (OtherActor :type "Actor Object Reference") (OtherComp :type "PrimitiveComponent Object Reference") (OtherBodyIndex :type Integer) (bFromSweep :type Boolean) (SweepResult :type "HitResult Structure (by ref)"))
  (bind _asbp_third_person_character (cast `/Game/Blueprints/BP_ThirdPersonCharacter` OtherActor))
  (`Character.LaunchCharacter` _asbp_third_person_character (* (4000.0 4000.0 500.0) (`KismetMathLibrary.Normal` (- (`self.K2_GetActorLocation` _asbp_third_person_character) (`self.K2_GetActorLocation`)))) false false))

(event `self.Capsule1.OnComponentBeginOverlap`
  (params (OverlappedComponent :type "PrimitiveComponent Object Reference") (OtherActor :type "Actor Object Reference") (OtherComp :type "PrimitiveComponent Object Reference") (OtherBodyIndex :type Integer) (bFromSweep :type Boolean) (SweepResult :type "HitResult Structure (by ref)"))
  (bind _asbp_third_person_character (cast `/Game/Blueprints/BP_ThirdPersonCharacter` OtherActor))
  (`Character.LaunchCharacter` _asbp_third_person_character (* (4000.0 4000.0 500.0) (`KismetMathLibrary.Normal` (- (`self.K2_GetActorLocation` _asbp_third_person_character) (`self.K2_GetActorLocation`)))) false false))

(fn `UserConstructionScript`)