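; Buildable item made of six mesh pieces that scatter at BeginPlay and hop at random via repeated physics impulses until built.
; An overlap radius tells BPI_Player actors when they can build it.
; While building, a timeline moves each piece in turn to its stored transform with physics off, and stopping halts the timeline.
; When all are placed, it gives the builder an item component and destroys itself.
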(event `PieceHop`
  (bind _scatteredpiecearray (`self.ScatteredPieceArray`))
  (bind _returnvalue (`KismetArrayLibrary.Array_Length` _scatteredpiecearray))
  (if (> _returnvalue 0)
    (`PrimitiveComponent.AddImpulse` (`|GetArrayItem` _scatteredpiecearray (`KismetMathLibrary.RandomIntegerInRange` 0 (- _returnvalue 1))) (0.0 0.0 10000.0) "None" false)
    (`KismetSystemLibrary.Delay` 0.5)
    (`self.PieceHop`)))

(event `self.ReceiveBeginPlay`
  (bind _returnvalue (`KismetMathLibrary.RandomFloatInRange` -120.0 120.0))
  (set `self.ScatteredPieceArray` (`|MakeArray` (`self.StaticMesh`) (`self.StaticMesh1`) (`self.StaticMesh2`) (`self.StaticMesh3`) (`self.StaticMesh4`) (`self.StaticMesh5`)))
  (for (_array_element _array_index) (`self.ScatteredPieceArray`)
    (`SceneComponent.K2_SetRelativeLocationAndRotation` _array_element (`KismetMathLibrary.MakeVector` (+ (.x (`|GetArrayItem` (`self.PieceLocationArray`) _array_index)) _returnvalue) (+ (.y (`|GetArrayItem` (`self.PieceLocationArray`) _array_index)) _returnvalue) (.z (`|GetArrayItem` (`self.PieceLocationArray`) _array_index))) (`KismetMathLibrary.RandomRotator` false) true false))
  (`KismetSystemLibrary.Delay` 5.0)
  (`self.PieceHop`))

(event `self.ReceiveActorBeginOverlap`
  (params (OtherActor :type "Actor Object Reference")))

(event `StopBuilding`
  (bind _output (`|GetArrayItem` (`self.ScatteredPieceArray`)))
  (set `self.Building?` false)
  (bind (_direction _alpha) (`Timeline|PieceMoveTimeline` :!via `Stop` :!label _label)
    (:`Update`
      (`SceneComponent.K2_SetRelativeLocationAndRotation` _output (`KismetMathLibrary.VLerp` (`self.Relative Location`) (+ (`|GetArrayItem` (`self.PieceLocationArray`) (`self.PiecesPlaced`)) (`self.K2_GetActorLocation`)) _alpha) (`KismetMathLibrary.RLerp` (`self.Relative Rotation`) (`|GetArrayItem` (`self.PieceRotationArray`) (`self.PiecesPlaced`)) _alpha) false false))
    (:`Finished`
      (`KismetArrayLibrary.Array_Add` (`self.PlacedPieceArray`) _output)
      (`KismetArrayLibrary.Array_Remove` (`self.ScatteredPieceArray`))
      (`/Engine/EditorBlueprintResources/StandardMacros.IncrementInt` (`self.PiecesPlaced`)
        (:`  `
          (if (`KismetArrayLibrary.Array_IsEmpty` (`self.ScatteredPieceArray`))
            (message `/Game/Blueprints/Interfaces/BPI_Player.AddItemComponent` (`self.Building Player Ref`) (`self.ItemComponentClass`))
            (`self.K2_DestroyActor`)
            (else
              (set `self.Relative Location` (`SceneComponent.RelativeLocation` _output) :!label _label_2)
              (set `self.Relative Rotation` (`SceneComponent.RelativeRotation` _output))
              (`PrimitiveComponent.SetSimulatePhysics` _output false)
              (goto _label :!via `PlayFromStart`))))))))

(event `self.Build Radius.OnComponentBeginOverlap`
  (params (OverlappedComponent :type "PrimitiveComponent Object Reference") (OtherActor :type "Actor Object Reference") (OtherComp :type "PrimitiveComponent Object Reference") (OtherBodyIndex :type Integer) (bFromSweep :type Boolean) (SweepResult :type "HitResult Structure (by ref)"))
  (if (`KismetSystemLibrary.DoesImplementInterface` OtherActor "/Game/Blueprints/Interfaces/BPI_Player.BPI_Player_C")
    (bind _output_get (set `self.LastOverlappingPlayer` OtherActor))
    (message `/Game/Blueprints/Interfaces/BPI_Player.CanBuildItem` _output_get true self)))

(event `StartBuilding`
  (params (`Building Player Ref` :type "/Game/Blueprints/BP_ThirdPersonCharacter Object Reference"))
  (if (not (`self.Building?`))
    (bind _output_get (set `self.Building Player Ref` `Building Player Ref`))
    (set `/Game/Blueprints/BP_ThirdPersonCharacter.Building` true _output_get)
    (set `self.Building?` true)
    (`/Engine/EditorBlueprintResources/StandardMacros.IsValid` (`|GetArrayItem` (`self.ScatteredPieceArray`))
      (:`Is Valid`
        (goto _label_2)))))

(event `self.Build Radius.OnComponentEndOverlap`
  (params (OverlappedComponent :type "PrimitiveComponent Object Reference") (OtherActor :type "Actor Object Reference") (OtherComp :type "PrimitiveComponent Object Reference") (OtherBodyIndex :type Integer))
  (bind _lastoverlappingplayer (`self.LastOverlappingPlayer`))
  (if (== OtherActor _lastoverlappingplayer)
    (message `/Game/Blueprints/Interfaces/BPI_Player.CanBuildItem` _lastoverlappingplayer false self)))

(fn `UserConstructionScript`)