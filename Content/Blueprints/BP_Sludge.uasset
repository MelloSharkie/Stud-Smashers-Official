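; BP_Sludge is a moving sludge hazard that slows and kills third-person characters.
; On BeginPlay it waits, then a timeline moves it from start to end location, and a later delay switches all characters off their primary spawns.
; An endless delayed loop spawns bubble Niagara effects at random points across its surface.
; Killbox overlap triggers death, while Slowbox lowers walk speed, gravity and jump until exit restores fixed values.
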(event `self.ReceiveBeginPlay`
  (`|ExecutionSequence`
    (:`then_0`
      (`KismetSystemLibrary.Delay` 28.0)
      (bind (_direction _alpha) (`Timeline|Timeline` :!via `PlayFromStart`)
        (:`Update`
          (`self.K2_SetActorLocation` (`KismetMathLibrary.VLerp` (`self.StartLocation`) (`self.EndLocation`) _alpha)))))
    (:`then_1`
      (`KismetSystemLibrary.Delay` 53.0)
      (bind _outactors (`GameplayStatics.GetAllActorsOfClass` "/Game/Blueprints/BP_ThirdPersonCharacter.BP_ThirdPersonCharacter_C"))
      (for _array_element _outactors
        (set `/Game/Blueprints/BP_ThirdPersonCharacter.UsePrimarySpawns?` false _array_element)))
    (:`then_2`
      (`NiagaraFunctionLibrary.SpawnSystemAtLocation` "/Game/VFX/N_Bubble.N_Bubble" (`KismetMathLibrary.RandomPointInBoundingBox` (`self.K2_GetActorLocation`) (750.0 1600.0 1.0)) :!label _label)
      (`KismetSystemLibrary.Delay` 0.1)
      (goto _label))))

(event `self.Killbox.OnComponentBeginOverlap`
  (params (OverlappedComponent :type "PrimitiveComponent Object Reference") (OtherActor :type "Actor Object Reference") (OtherComp :type "PrimitiveComponent Object Reference") (OtherBodyIndex :type Integer) (bFromSweep :type Boolean) (SweepResult :type "HitResult Structure (by ref)"))
  (bind _asbp_third_person_character (cast `/Game/Blueprints/BP_ThirdPersonCharacter` OtherActor))
  (`/Game/Blueprints/BP_ThirdPersonCharacter.Trigger Death` _asbp_third_person_character))

(event `self.Slowbox.OnComponentBeginOverlap`
  (params (OverlappedComponent :type "PrimitiveComponent Object Reference") (OtherActor :type "Actor Object Reference") (OtherComp :type "PrimitiveComponent Object Reference") (OtherBodyIndex :type Integer) (bFromSweep :type Boolean) (SweepResult :type "HitResult Structure (by ref)"))
  (bind _asbp_third_person_character (cast `/Game/Blueprints/BP_ThirdPersonCharacter` OtherActor))
  (bind _charactermovement (`Character.CharacterMovement` _asbp_third_person_character))
  (`MovementComponent.StopMovementImmediately` _charactermovement)
  (set `CharacterMovementComponent.MaxWalkSpeed` 300.0 _charactermovement)
  (set `CharacterMovementComponent.GravityScale` 0.1 _charactermovement)
  (set `CharacterMovementComponent.JumpZVelocity` 300.0 _charactermovement))

(event `self.Slowbox.OnComponentEndOverlap`
  (params (OverlappedComponent :type "PrimitiveComponent Object Reference") (OtherActor :type "Actor Object Reference") (OtherComp :type "PrimitiveComponent Object Reference") (OtherBodyIndex :type Integer))
  (bind _asbp_third_person_character (cast `/Game/Blueprints/BP_ThirdPersonCharacter` OtherActor))
  (bind _charactermovement (`Character.CharacterMovement` _asbp_third_person_character))
  (set `CharacterMovementComponent.MaxWalkSpeed` 600.0 _charactermovement)
  (set `CharacterMovementComponent.GravityScale` 2.2 _charactermovement)
  (set `CharacterMovementComponent.JumpZVelocity` 750.0 _charactermovement))

(fn `UserConstructionScript`)