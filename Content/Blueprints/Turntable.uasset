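; Turntable Blueprint that showcases animations on a skeletal mesh by playing the entries of an array in sequence.
; From BeginPlay, a custom event plays the current entry without looping, waits a short fixed delay, increments the index and calls itself again through that delayed loop.
; The index is clamped to a hard-coded maximum rather than wrapped, so the animation at that last index restarts repeatedly.
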(event `self.ReceiveBeginPlay`
  (`self.Showcase Animations` :!label _label))

(event `Showcase Animations`
  (`SkeletalMeshComponent.PlayAnimation` (`self.SkeletalMesh`) (`|GetArrayItem` (`self.animationArray`) (`self.AnimationToPlay`)) false)
  (`KismetSystemLibrary.Delay` 0.8)
  (set `self.AnimationToPlay` (`KismetMathLibrary.Clamp` (+ (`self.AnimationToPlay`) 1) 0 16))
  (goto _label))

(fn `UserConstructionScript`)