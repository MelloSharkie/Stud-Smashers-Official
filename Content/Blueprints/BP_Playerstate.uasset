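; Player state Blueprint that stores a player's character selection and carries PlayerProfile over to a new player state through CopyProperties.
; SetPlayerCharacter caches the character, franchise, integer and a reference.
; SetPlayerCharacterOnServer forwards to SetPlayerCharacterOnClient, which sends AssignPlayerCharacterMessage to the passed reference.
; SetPlayerCharacter does not trigger that chain: its call is disconnected, and OnRep_Integer is empty apart from unreachable nodes.
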(event `self.ReceiveCopyProperties`
  (params (NewPlayerState :type "PlayerState Object Reference"))
  (bind _asbp_playerstate (cast `/Game/Blueprints/BP_Playerstate` NewPlayerState))
  (set `/Game/Blueprints/BP_Playerstate.Player Profile` (`self.Player Profile`) _asbp_playerstate))

(event `Set Player Character`
  (params (`Character STR` :type "/Game/Blueprints/Variables/STR_Characters Structure") (`Franchise ENUM` :type "/Game/Blueprints/Variables/E_Franchise Enum" :default "NewEnumerator0") (Integer :type Integer) (`Self REF` :type "/Game/Blueprints/BP_ThirdPersonCharacter Object Reference"))
  (set `self.Character STR` `Character STR`)
  (set `self.Franchise ENUM` `Franchise ENUM`)
  (set `self.Self REF` `Self REF`)
  (set `self.Integer` Integer))

(event `Set Player Character On Server`
  (params (`Self Ref` :type "/Game/Blueprints/BP_ThirdPersonCharacter Object Reference") (Integer :type Integer))
  (`self.Set Player Character On Client` `Self Ref` Integer))

(event `Set Player Character On Client`
  (params (`Self Ref` :type "/Game/Blueprints/BP_ThirdPersonCharacter Object Reference") (Integer :type Integer))
  (message `/Game/Blueprints/Interfaces/BPI_Player.Assign Player Character ` `Self Ref` (struct) Integer `Self Ref`))

(fn `OnRep_Integer`)

(fn `UserConstructionScript`)