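; BP_GrabTether is a tether Blueprint that gathers movement input from the players in its TetheredPlayers array.
; Each Tick it fetches every player's move input message and adds X and Y into TotalXInput and TotalYInput.
; The totals are never reset or applied here, and the divisions that would average them by player count are unconnected.
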(event `self.ReceiveTick`
  (params (DeltaSeconds :type "Float (single-precision)"))
  (for _array_element (`self.TetheredPlayers`)
    (bind (_x _y) (message `/Game/Blueprints/Interfaces/BPI_Player.FetchMoveInput` _array_element))
    (set `self.TotalXInput` (+ _x (`self.TotalXInput`)))
    (set `self.TotalYInput` (+ _y (`self.TotalYInput`)))))

(fn `UserConstructionScript`)