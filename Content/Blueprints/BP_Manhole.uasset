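; Manhole actor that periodically builds steam pressure and erupts, shaking and then launching its cover mesh upward.
; A delay loop started on BeginPlay increments a pressure counter while inactive, and ValveSpun enters the same check immediately to add pressure.
; At the threshold, a shake timeline hands off to Niagara steam and a timeline moving and tilting the cover.
; A timed delay then stops the steam and clears Active.
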(event `self.ReceiveBeginPlay`
  (`KismetSystemLibrary.Delay` 8.0)
  (`KismetSystemLibrary.Delay` 3.0 :!label _label)
  (if (`self.Active?`) :!label _label_2
    (goto _label)
    (else
      (bind _result (`/Engine/EditorBlueprintResources/StandardMacros.IncrementInt` (`self.PressureBuilt`))
        (:`  `
          (if (>= _result 5)
            (set `self.PressureBuilt` 0)
            (`self.ActivateSteam`)
            (goto _label)
            (else
              (goto _label))))))))

(event `/Game/Blueprints/Interfaces/BPI_Valve.ValveSpun`
  (goto _label_2))

(event `ActivateSteam`
  (bind _niagara (`self.Niagara`))
  (bind _staticmesh (`self.StaticMesh`))
  (bind _manholestartlocation (`self.ManholeStartLocation`))
  (set `self.Active?` true)
  (bind (_direction _rotationalalpharoll _rotationalalphapitch) (`Timeline|ShakingManhole` :!via `PlayFromStart`)
    (:`Update`
      (`SceneComponent.K2_SetRelativeRotation` (`self.StaticMesh`) (`KismetMathLibrary.MakeRotator` (`KismetMathLibrary.Lerp` 0.0 50.0 _rotationalalpharoll) (`KismetMathLibrary.Lerp` 0.0 50.0 _rotationalalphapitch)) false false))
    (:`Finished`
      (`ActorComponent.Activate` _niagara true)
      (`|ExecutionSequence`
        (:`then_0`
          (set `self.ManholeStartLocation` (`SceneComponent.K2_GetComponentLocation` _staticmesh))
          (bind (_direction_2 _locationalpha _rotationalpharoll _rotationalphapitch) (`Timeline|RisingManholeTimeline` :!via `PlayFromStart`)
            (:`Update`
              (`SceneComponent.K2_SetWorldLocation` _staticmesh (`KismetMathLibrary.VLerp` _manholestartlocation (+ _manholestartlocation (0.0 0.0 596.8)) _locationalpha) false false)
              (`SceneComponent.K2_SetRelativeRotation` (`self.StaticMesh`) (`KismetMathLibrary.MakeRotator` (`KismetMathLibrary.Lerp` 0.0 50.0 _rotationalpharoll) (`KismetMathLibrary.Lerp` 0.0 50.0 _rotationalphapitch)) false false))))
        (:`then_1`
          (`KismetSystemLibrary.Delay` 6.0)
          (`ActorComponent.Deactivate` _niagara)
          (set `self.Active?` false))))))

(fn `UserConstructionScript`)